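; Test actor that swaps its static mesh material when something enters or leaves its box.
; Box overlap begin applies burnished steel; overlap end restores the base M_Chair material, not the dynamic instance.
; The construction script creates a dynamic M_Chair instance, whose "Chair" color parameter turns black on actor overlap, though box swaps replace that instance on the mesh.
; BeginPlay prints a debug message.
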(event OnComponentEndOverlap(Box)
  (params (OtherActor :type Actor%20Object%20Reference) (OtherComp :type Primitive%20Component%20Object%20Reference) (OtherBodyIndex :type Integer))
  (Rendering|Material|SetMaterial (Variables|Default|GetStaticMesh) 0 "/Game/StarterContent/Props/Materials/M_Chair.M_Chair"))

(event OnComponentBeginOverlap(Box)
  (params (OtherActor :type Actor%20Object%20Reference) (OtherComp :type Primitive%20Component%20Object%20Reference) (OtherBodyIndex :type Integer) (bFromSweep :type Boolean) (SweepResult :type Hit%20Result%20Structure%20%28by%20ref%29))
  (Rendering|Material|SetMaterial (Variables|Default|GetStaticMesh) 0 "/Game/StarterContent/Materials/M_Metal_Burnished_Steel.M_Metal_Burnished_Steel"))

(event EventBeginPlay
  (Development|PrintText "pepe's here"))

(event EventActorBeginOverlap
  (params (OtherActor :type Actor%20Object%20Reference))
  (Rendering|Material|SetVectorParameterValue :self (Variables|Default|Getvariable) :ParameterName "Chair" :!class /Script/Engine.MaterialInstanceDynamic))

(event EventTick
  (params (DeltaSeconds :type Float%20%28single-precision%29)))

(fn ConstructionScript
  (bind _returnvalue (Rendering|Material|CreateDynamicMaterialInstance (Variables|Default|GetStaticMesh) 0 "/Game/StarterContent/Props/Materials/M_Chair.M_Chair" :!class /Script/Engine.PrimitiveComponent))
  (Variables|Default|Setvariable _returnvalue))